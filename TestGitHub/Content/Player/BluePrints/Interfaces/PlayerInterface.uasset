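; Blueprint interface for the player, exposing animation-related state and an item pickup call without declaring any logic of its own.
; Getters return the left socket transform, hand sway inputs from side movement and mouse, aim state, left-hand tracking stop flag, wall distance and an animation state enum.
; IFAddItem passes an item and its pickup to the implementer.
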(fn IFGetLeftSocketTransform
  (return ""))

(fn IFGetHandSwayFloats
  (return 0.0 0.0 0.0))

(fn IFGetAim
  (return false))

(fn IFStopLeftHandTracking
  (return false))

(fn IFGetWallDistance
  (return 0.0))

(fn IFAddItem
  (params (Item :type Dynamic%20Inventory%20Item%20Structure) (PickUp :type Actor%20Object%20Reference)))

(fn IFGetAnimState
  (return "NewEnumerator0"))